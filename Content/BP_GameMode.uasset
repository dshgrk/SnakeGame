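; Game mode for a grid-based Snake game that runs the match from start screen or instant restart through to death.
; SetUp spawns the ground grid, first tail box and food.
; A looping timer calls UpdateTail, which advances a position array by Direction, repositions the boxes, and handles eating, growth and score.
; Leaving the hard-coded bounds or hitting the body stops the timer, shows the death widget and records the score through BP_Restarting.
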(event `self.ReceiveBeginPlay`
  (bind _returnvalue (`GameplayStatics.GetPlayerController` 0))
  (bind _asbp_restarting (cast `/Game/BP_Restarting` (`GameplayStatics.GetGameInstance`)))
  (if (`/Game/BP_Restarting.Restarting` _asbp_restarting)
    (`self.StartGame`)
    (else
      (bind _returnvalue_2 (`|CreateWidget` "/Game/WBP_Start.WBP_Start_C"))
      (`UserWidget.AddToViewport` _returnvalue_2 0)
      (`WidgetBlueprintLibrary.SetInputMode_UIOnlyEx` _returnvalue _returnvalue_2)
      (set `PlayerController.bShowMouseCursor` true _returnvalue)))
  (bind _returnvalue_3 (`|CreateWidget` "/Game/WBP_Score.WBP_Score_C"))
  (bind _output_get (set `self.ScoreUI` _returnvalue_3))
  (`UserWidget.AddToViewport` _output_get 0))

(fn `Can Go To Position?`
  (params (Position :type "Vector Structure"))
  (returns (`Can Go To Position` :type Boolean))
  (locals (positionHead :type "Vector Structure") (`can go` :type Boolean :default true))
  (bind _output_get (set `local.positionHead` Position))
  ; check can go to next cube
  (if (`KismetMathLibrary.BooleanNOR` (xor (< (.x _output_get) 0.0) (> (.x _output_get) 29.0)) (xor (< (.y _output_get) 0.0) (> (.y _output_get) 29.0)))
    ; check head is in body
    (for _array_element (`self.TailPositions`)
      (if (`KismetMathLibrary.EqualExactly_VectorVector` _array_element (`local.positionHead`))
        (set `local.can go` false)))
    (return (`local.can go`))
    (else
      (return false))))

(fn `Death`
  (bind _returnvalue (`GameplayStatics.GetPlayerController` 0))
  (`KismetSystemLibrary.K2_ClearAndInvalidateTimerHandle` (`self.Timer`))
  (bind _returnvalue_2 (`|CreateWidget` "/Game/WBP_Death.WBP_Death_C"))
  (bind _output_get (set `self.DeathUI` _returnvalue_2))
  (`UserWidget.AddToViewport` _output_get 0)
  (`WidgetBlueprintLibrary.SetInputMode_UIOnlyEx` _returnvalue (`self.DeathUI`) "DoNotLock" true)
  (set `PlayerController.bShowMouseCursor` true _returnvalue)
  (bind _asbp_restarting (cast `/Game/BP_Restarting` (`GameplayStatics.GetGameInstance`)))
  (`/Game/BP_SaveGame.Add Result` (`/Game/BP_Restarting.SaveGameRef` _asbp_restarting) (`self.Score`)))

(fn `Grow`
  (params (Position :type "Vector Structure"))
  (`KismetArrayLibrary.Array_Insert` (`self.TailPositions`) Position)
  (bind _returnvalue (`|SpawnActorFromClass` "/Game/BP_Tail.BP_Tail_C" (`KismetMathLibrary.MakeTransform` (* Position (`self.Scale`))) "Undefined" "MultiplyWithRoot" null null))
  (`KismetArrayLibrary.Array_Add` (`self.TailBoxes`) _returnvalue))

(fn `Random Food Position`
  (returns (`Random Food Position` :type "Vector Structure"))
  (set `self.RandomFoodPosition` (`KismetMathLibrary.MakeVector` (`KismetMathLibrary.Conv_IntToDouble` (`KismetMathLibrary.RandomIntegerInRange` 1 (- (`self.Height`) 2))) (`KismetMathLibrary.Conv_IntToDouble` (`KismetMathLibrary.RandomIntegerInRange` 1 (- (`self.Height`) 2)))))
  (return (`self.RandomFoodPosition`)))

(fn `SetUp`
  (locals (Y :type Integer) (X :type Integer))
  (`|ExecutionSequence`
    (:`then_0`
      ; Setup Grid Ground
      (for _index (range (`self.Height`))
        (set `local.Y` _index)
        (for _index_2 (range (`self.Width`))
          (set `local.X` _index_2)
          (`|SpawnActorFromClass` "/Game/BP_Ground.BP_Ground_C" (`KismetMathLibrary.MakeTransform` (`KismetMathLibrary.MakeVector` (`KismetMathLibrary.Conv_IntToDouble` (* (`local.X`) (`self.Scale`))) (`KismetMathLibrary.Conv_IntToDouble` (* (`local.Y`) (`self.Scale`))) (`KismetMathLibrary.Conv_IntToDouble` (* (`self.Scale`) -1)))) "Undefined" "MultiplyWithRoot" null null))))
    (:`then_1`
      ; setup tail
      (bind _output_get (set `self.StartPosition` (`KismetMathLibrary.MakeVector` (`KismetMathLibrary.Conv_IntToDouble` (/ (`self.Height`) 2)) (`KismetMathLibrary.Conv_IntToDouble` (/ (`self.Width`) 2)))))
      (`self.Grow` _output_get))
    (:`then_2`
      ; Setup Food
      (bind _random_food_position (`self.Random Food Position`))
      (bind (_returnvalue_x _returnvalue_y) (`KismetMathLibrary.BreakVector` (* _random_food_position (`self.Scale`))))
      (bind _returnvalue (`|SpawnActorFromClass` "/Game/BP_Food.BP_Food_C" (`KismetMathLibrary.MakeTransform` (`KismetMathLibrary.MakeVector` _returnvalue_x _returnvalue_y (`KismetMathLibrary.Conv_IntToDouble` (`self.Scale`)))) "Undefined" "MultiplyWithRoot" null null))
      (set `self.Food` _returnvalue))))

(fn `StartGame`
  (bind _returnvalue (`GameplayStatics.GetPlayerController` 0))
  (`self.SetUp`)
  (`WidgetBlueprintLibrary.SetInputMode_GameOnly` _returnvalue)
  (set `PlayerController.bShowMouseCursor` false _returnvalue)
  (`self.Update Timer`))

(fn `Update Timer`
  (`KismetSystemLibrary.K2_ClearAndInvalidateTimerHandle` (`self.Timer`))
  (bind _returnvalue (`KismetSystemLibrary.K2_SetTimer` null "UpdateTail" 0.2 true))
  (set `self.Timer` _returnvalue))

(fn `UpdateTail`
  (locals (NewFirstBoxPosition :type "Vector Structure"))
  (bind _tailpositions (`self.TailPositions`))
  ; find next head-box position
  (bind _output_get (set `local.NewFirstBoxPosition` (+ (`|GetArrayItem` (`self.TailPositions`)) (`self.Direction`))))
  ; game over
  (bind _can_go_to_position (`self.Can Go To Position?` _output_get))
  (if _can_go_to_position
    ; check for food
    (if (`KismetMathLibrary.EqualExactly_VectorVector` (`local.NewFirstBoxPosition`) (`self.RandomFoodPosition`))
      ; eat and grow
      (`self.Grow` (`local.NewFirstBoxPosition`))
      (bind _random_food_position (`self.Random Food Position`))
      (`self.K2_SetActorLocation` (`self.Food`) (`KismetMathLibrary.MakeVector` (* (.x _random_food_position) (`self.Scale`)) (* (.y _random_food_position) (`self.Scale`)) (`KismetMathLibrary.Conv_IntToDouble` (`self.Scale`))) false false)
      (bind _result (`/Engine/EditorBlueprintResources/StandardMacros.IncrementInt` (`self.Score`))
        (:`  `
          (`/Game/WBP_Score.Update Score` (`self.ScoreUI`) _result)
          (`self.Update Timer`)))
      (else
        ; just move
        (`KismetArrayLibrary.Array_Remove` _tailpositions (`KismetArrayLibrary.Array_LastIndex` _tailpositions))
        (`KismetArrayLibrary.Array_Insert` (`self.TailPositions`) (`local.NewFirstBoxPosition`))
        (for (_array_element _array_index) (`self.TailBoxes`)
          (`self.K2_SetActorLocation` _array_element (* (`|GetArrayItem` (`self.TailPositions`) _array_index) (`self.Scale`)) false false))))
    (else
      (`self.Death`))))

(fn `UserConstructionScript`)