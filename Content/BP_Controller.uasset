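; BP_Controller is the controller for a Snake game, turning player input into movement direction changes.
; BeginPlay adds the IMC_SnakeGame Enhanced Input mapping context, and four directional input actions each pass a unit axis vector to SetDirection.
; SetDirection rejects exact reversals of the current direction held in BP_GameMode, otherwise storing the new direction there and calling UpdateTail and UpdateTimer on the game mode.
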(event `self.ReceiveBeginPlay`
  (`EnhancedInputSubsystemInterface.AddMappingContext` (subsystem `EnhancedInputLocalPlayerSubsystem`) "/Game/Inputs/IMC_SnakeGame.IMC_SnakeGame" 0 (struct)))

(event `EnhancedInput|/Game/Inputs/IA_UP`
  (params (ActionValue :type Boolean) (ElapsedSeconds :type "Float (double-precision)") (TriggeredSeconds :type "Float (double-precision)") (InputAction :type "InputAction Object Reference" :default "/Game/Inputs/IA_UP.IA_UP"))
  (:`Started`
    (`self.Set Direction` (1.0 0.0 0.0))))

(event `EnhancedInput|/Game/Inputs/IA_DOWN`
  (params (ActionValue :type Boolean) (ElapsedSeconds :type "Float (double-precision)") (TriggeredSeconds :type "Float (double-precision)") (InputAction :type "InputAction Object Reference" :default "/Game/Inputs/IA_DOWN.IA_DOWN"))
  (:`Started`
    (`self.Set Direction` (-1.0 0.0 0.0))))

(event `EnhancedInput|/Game/Inputs/IA_RIGHT`
  (params (ActionValue :type Boolean) (ElapsedSeconds :type "Float (double-precision)") (TriggeredSeconds :type "Float (double-precision)") (InputAction :type "InputAction Object Reference" :default "/Game/Inputs/IA_RIGHT.IA_RIGHT"))
  (:`Started`
    (`self.Set Direction` (0.0 1.0 0.0))))

(event `EnhancedInput|/Game/Inputs/IA_LEFT`
  (params (ActionValue :type Boolean) (ElapsedSeconds :type "Float (double-precision)") (TriggeredSeconds :type "Float (double-precision)") (InputAction :type "InputAction Object Reference" :default "/Game/Inputs/IA_LEFT.IA_LEFT"))
  (:`Started`
    (`self.Set Direction` (0.0 -1.0 0.0))))

(fn `Set Direction`
  (params (`New Direction` :type "Vector Structure"))
  (bind _asbp_game_mode (cast `/Game/BP_GameMode` (`GameplayStatics.GetGameMode`)))
  (if (not (`KismetMathLibrary.EqualExactly_VectorVector` (* (`/Game/BP_GameMode.Direction` _asbp_game_mode) -1) `New Direction`))
    (set `/Game/BP_GameMode.Direction` `New Direction` _asbp_game_mode)
    (`/Game/BP_GameMode.UpdateTail` _asbp_game_mode)
    (`/Game/BP_GameMode.Update Timer` _asbp_game_mode)))

(fn `UserConstructionScript`)