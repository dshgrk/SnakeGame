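; GenerateTerain is a Blueprint that lays out a flat, grid-shaped terrain from instanced static meshes when play begins.
; BeginPlay runs nested loops over Height and Width, adding one InstancedStaticMesh instance per cell.
; Scale sets the X and Y spacing between cells and places the whole layer one Scale unit below zero on Z, with no height variation.
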(event `self.ReceiveBeginPlay`
  (for _index (range (`self.Height`))
    (set `self.Y` _index)
    (for _index_2 (range (`self.Width`))
      (set `self.X` _index_2)
      (`InstancedStaticMeshComponent.AddInstance` (`self.InstancedStaticMesh`) (`KismetMathLibrary.MakeTransform` (`KismetMathLibrary.MakeVector` (`KismetMathLibrary.Conv_IntToDouble` (* (`self.X`) (`self.Scale`))) (`KismetMathLibrary.Conv_IntToDouble` (* (`self.Y`) (`self.Scale`))) (`KismetMathLibrary.Conv_IntToDouble` (* (`self.Scale`) -1)))) false))))

(fn `UserConstructionScript`)