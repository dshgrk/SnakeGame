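; Initialization Blueprint that restores saved audio volume settings when its Init event runs.
; It loads BP_SaveGame from its save slot, or creates and saves a new one if none exists, keeping it in SaveGameRef.
; Both paths then set music, effects and overall sound class overrides on NewSoundMix, reading volumes from the load branch's cast result, even for a new save.
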(event `self.ReceiveInit`
  (bind _slotname (`self.SlotName`))
  (bind _returnvalue (`GameplayStatics.DoesSaveGameExist` _slotname))
  (if _returnvalue
    (bind _returnvalue_2 (`GameplayStatics.LoadGameFromSlot` _slotname))
    (bind _asbp_save_game (cast `/Game/Blueprints/BP_SaveGame` _returnvalue_2))
    (set `self.SaveGameRef` _asbp_save_game)
    (else
      (bind _returnvalue_3 (`GameplayStatics.CreateSaveGameObject` "/Game/Blueprints/BP_SaveGame.BP_SaveGame_C"))
      (bind _output_get (set `self.SaveGameRef` _returnvalue_3))
      (`GameplayStatics.SaveGameToSlot` _output_get _slotname)))
  (`GameplayStatics.SetSoundMixClassOverride` "/Game/Sounds/NewSoundMix.NewSoundMix" "/Game/Sounds/SC_Music.SC_Music" (`/Game/Blueprints/BP_SaveGame.MusicVolume` _asbp_save_game))
  (`GameplayStatics.SetSoundMixClassOverride` "/Game/Sounds/NewSoundMix.NewSoundMix" "/Game/Sounds/SC_FX.SC_FX" (`/Game/Blueprints/BP_SaveGame.EffectsVolume` _asbp_save_game))
  (`GameplayStatics.SetSoundMixClassOverride` "/Game/Sounds/NewSoundMix.NewSoundMix" "/Game/Sounds/SC_ALL.SC_ALL" (`/Game/Blueprints/BP_SaveGame.AllVolume` _asbp_save_game)))